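; Ship controller that drives a physics "Driver" component from throttle and turn values, with debug keyboard axis input.
; A looping timer steps forward throttle by acceleration, either from input or toward a clamped target.
; Tick applies counter-torque to damp spin, lerps velocity toward the throttle-scaled forward vector, and adds yaw torque.
; Vertical throttle logic is unfinished: it is never called and reuses forward limits.
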(event `self.ReceiveBeginPlay`
  ;[1 1 1] Update Foward
  (`KismetSystemLibrary.K2_SetTimer` null "UpdateForwardThrottle" (`self.UpdateThrottleTickRate`) true))

(event `InputAxis|ShipForward`
  (params (AxisValue :type "Float (single-precision)"))
  ;[1 0.4493 0.3695] Debug Forward Manual Keyboard Input
  (set `self.ForwardThrottleInput` AxisValue))

(event `self.ReceiveTick`
  (params (DeltaSeconds :type "Float (single-precision)"))
  ;[1 1 1] Update Physics
  (`PrimitiveComponent.AddTorqueInDegrees` (`self.Driver`) (/ (`KismetMathLibrary.NegateVector` (`PrimitiveComponent.GetPhysicsAngularVelocityInDegrees` (`self.Driver`) "None")) 0.5) "None" true)
  (`self.UpdateCalculatedSpeed`)
  ;[1 1 1] Update Turn w/ Debug Turn Manual Keyboard Input
  (set `self.TurnInput` (stale `InputAxis|ShipRight` AxisValue) :!label _label)
  (`self.UpdateTurning`))

(event `InputAxis|ShipRight`
  (params (AxisValue :type "Float (single-precision)"))
  ;[1 1 1] Update Turn w/ Debug Turn Manual Keyboard Input
  (goto _label))

(fn `UpdateCalculatedSpeed`
  (bind _driver (`self.Driver`))
  (bind _returnvalue (`PrimitiveComponent.GetPhysicsLinearVelocity` _driver "None"))
  (`PrimitiveComponent.SetPhysicsLinearVelocity` (`self.Driver`) (`KismetMathLibrary.VLerp` _returnvalue (* (`SceneComponent.GetForwardVector` _driver) (* (`self.ForwardThrottleAmount`) (`self.UE4_ForceConstant`))) 0.01) false "None"))

(fn `UpdateForwardThrottle`
  (bind _forwardtargetthrottle (`self.ForwardTargetThrottle`))
  (bind _maxreversethrottle (`self.MaxReverseThrottle`))
  (bind _maxforwardthrottle (`self.MaxForwardThrottle`))
  (bind _forwardtargetthrottle_2 (`self.ForwardTargetThrottle`))
  (bind _forwardthrottleamount (`self.ForwardThrottleAmount`))
  (bind _returnvalue (+ (* (`self.ForwardThrottleInput`) (`self.ForwardAcceleration`)) (`self.ForwardThrottleAmount`)))
  ;[1 1 1] Clamp Initial Target Value
  (set `self.ForwardTargetThrottle` (`KismetMathLibrary.FClamp` (`self.ForwardTargetThrottle`) (`self.MaxReverseThrottle`) (`self.MaxForwardThrottle`)))
  ;[0.7975 0.4754 1] Forward Target Throttle Value is being Used
  (if (== (`self.UseForwardTargetThrottle`) true)
    ;[0.4588 0.6941 1] Set Forward Input depending on the direction Throttle Amount needs to catch-up to Target Throttle
    (if (== _forwardtargetthrottle _forwardthrottleamount)
      (set `self.ForwardThrottleInput` 0.0)
      ;[1 0.4583 0.4583] Simple Forward Throttle Update
      (bind _output_get (set `self.ForwardThrottleAmount` (`KismetMathLibrary.FClamp` _returnvalue _maxreversethrottle _maxforwardthrottle) :!label _label))
      (elif (> _forwardtargetthrottle _forwardthrottleamount)
        (set `self.ForwardThrottleInput` 1.0)
        ;[0.4588 0.6941 1] Update Forward Throttle to its progress towards the Target, and also clamp it to the target
        (set `self.ForwardThrottleAmount` (`KismetMathLibrary.FClamp` _returnvalue _maxreversethrottle _forwardtargetthrottle_2))
        (else
          (set `self.ForwardThrottleInput` -1.0)
          (set `self.ForwardThrottleAmount` (`KismetMathLibrary.FClamp` _returnvalue _forwardtargetthrottle_2 _maxforwardthrottle)))))
    (else
      (goto _label)))
  ;[1 1 1] Debug Print
  (`KismetSystemLibrary.PrintString` (`KismetStringLibrary.Conv_DoubleToString` _output_get) true true (struct :`R` 1.0 :`G` 0.184235 :`B` 0.253958 :`A` 1.0)))

(fn `UpdateTurning`
  (bind _driver (`self.Driver`))
  (`PrimitiveComponent.AddTorqueInDegrees` _driver (`KismetMathLibrary.VLerp` (0.0 0.0 0.0) (* (`SceneComponent.GetUpVector` _driver) (* (`self.TurnInput`) (`self.TurnSpeed`))) (`self.TurnLerpAlpha`)) "None" true))

(fn `UpdateVerticalThrottle`
  (bind _verticaltargetthrottle (`self.VerticalTargetThrottle`))
  (bind _maxreversethrottle (`self.MaxReverseThrottle`))
  (bind _verticalthrottleamount (`self.VerticalThrottleAmount`))
  (bind _maxforwardthrottle (`self.MaxForwardThrottle`))
  (bind _forwardtargetthrottle (`self.ForwardTargetThrottle`))
  (bind _returnvalue (+ (* (`self.VerticalTargetThrottle`) (`self.VerticalAcceleration`)) (`self.VerticalThrottleAmount`)))
  ;[1 1 1] Clamp Initial Target Value
  (set `self.VerticalTargetThrottle` (`KismetMathLibrary.FClamp` (`self.VerticalTargetThrottle`) (`self.MaxDownThrottle`) (`self.MaxUpThrottle`)))
  ;[0.7975 0.4754 1] Forward Target Throttle Value is being Used
  (if (== (`self.UseVerticalTargetThrottle`) true)
    ;[0.4588 0.6941 1] Set Forward Input depending on the direction Throttle Amount needs to catch-up to Target Throttle
    (if (== _verticaltargetthrottle _verticalthrottleamount)
      (set `self.VerticalThrottleInput` 0.0)
      ;[1 0.4583 0.4583] Simple Forward Throttle Update
      (bind _output_get (set `self.VerticalTargetThrottle` (`KismetMathLibrary.FClamp` _returnvalue _maxreversethrottle _maxforwardthrottle) :!label _label))
      (elif (> _verticaltargetthrottle _verticalthrottleamount)
        (set `self.VerticalThrottleInput` 1.0)
        ;[0.4588 0.6941 1] Update Forward Throttle to its progress towards the Target, and also clamp it to the target
        (set `self.VerticalTargetThrottle` (`KismetMathLibrary.FClamp` _returnvalue _maxreversethrottle _forwardtargetthrottle))
        (else
          (set `self.VerticalThrottleInput` -1.0)
          (set `self.VerticalTargetThrottle` (`KismetMathLibrary.FClamp` _returnvalue _forwardtargetthrottle _maxforwardthrottle)))))
    (else
      (goto _label)))
  ;[1 1 1] Debug Print
  (`KismetSystemLibrary.PrintString` (`KismetStringLibrary.Conv_DoubleToString` _output_get) true true (struct :`R` 1.0 :`G` 0.184235 :`B` 0.253958 :`A` 1.0)))

(fn `UserConstructionScript`)